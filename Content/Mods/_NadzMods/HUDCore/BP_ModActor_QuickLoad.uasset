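; HUDCore mod actor that quick-loads straight into a solo game when it begins play.
; BeginPlay asks the game state machine for a random level at the first difficulty index, with pre-match skipped.
; ParseHUDData and AddSettingsStackToMenu are empty; leftover HUD settings save/load nodes in ParseHUDData never run.
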(event EventBeginPlay
  (|CallParentFunction)
  (Class|SBZGameStateMachine|RequestSoloGame (Class|SBZGameStateMachineFunctionLibrary|GetGameStateMachine) (Math|Random|RandomIntegerinRange 0 (- (Utilities|Array|Length (Class|SBZGameStateMachineSettings|GetLevels)) 1)) 0 true))

(fn ConstructionScript
  (|CallParentFunction))

(fn ParseHUDData
  (params (DA :type PDA%20Custom%20HUD%20Object%20Reference)))

(fn AddSettingsStacktoMenu)