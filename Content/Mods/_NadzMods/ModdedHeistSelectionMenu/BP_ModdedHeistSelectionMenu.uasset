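; Mod actor for a modded heist selection menu, creating the menu widget at BeginPlay and adding it to the viewport collapsed.
; Helper functions find non-tutorial heists absent from game collections, build banner buttons mapped to their data, and show descriptions with stealth/loud best times.
; Only widget creation is live: list building, selection and solo-game launch are disconnected, and both button events and time-text array setters are empty.
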(event Custom|OnHeistButtonSelected
  (params (Button :type SBZ%20Menu%20Button%20Object%20Reference)))

(event Custom|OnButtonHover
  (params (Button :type SBZ%20Menu%20Button%20Object%20Reference) (bIsEnabled :type Boolean)))

(event EventBeginPlay
  (bind _returnvalue (UserInterface|CreateWidget "/Game/Mods/_NadzMods/ModdedHeistSelectionMenu/UI/WBP_UI_ModdedHeistsSelection.WBP_UI_ModdedHeistsSelection_C"))
  (bind _output_get (Variables|Default|SetModdedHeistsMenu _returnvalue))
  (UserInterface|Viewport|AddtoViewport _output_get 0)
  (Widget|SetVisibility _output_get "Collapsed"))

(fn ConstructionScript)

(fn GetHeistInfo
  (Utilities|FlowControl|Sequence
    (:then_0
      (for _array_element (Class|SBZGameStateMachineSettings|GetHeistCollections)
        (for _array_element_2 (.LevelPaths (Utilities|Struct|BreakSBZHeistCollection _array_element))
          (Utilities|Array|AddUnique (Variables|Default|GetGameHeistsLevelPaths) _array_element_2))))
    (:then_1
      (for _array_element_3 (Class|SBZHeistDeveloperSettings|GetAllHeistData)
        (if (not (or (Utilities|Array|ContainsItem (Variables|Default|GetGameHeistsLevelPaths) (.LevelPath (Utilities|Struct|BreakSBZHeistDataLevelPair _array_element_3))) (Utilities|String|Contains (Utilities|BreakSoftObjectPath (.LevelPath (Utilities|Struct|BreakSBZHeistDataLevelPair _array_element_3))) "/Game/Prototype/Maps/Tutorial")))
          (Utilities|Array|AddUnique (Variables|Default|GetModdedHeistsArray) _array_element_3)
          (Utilities|Array|AddUnique (Variables|Default|GetLevelPaths) (.LevelPath (Utilities|Struct|BreakSBZHeistDataLevelPair _array_element_3))))))))

(fn MakeModdedHeistButtons
  (for _array_element (Variables|Default|GetModdedHeistsArray)
    (bind _returnvalue (UserInterface|CreateWidget "/Game/UI/Widgets/Menus/Buttons/WBP_UI_CrimeNet_TextButton.WBP_UI_CrimeNet_TextButton_C"))
    (Default|SetButtonText _returnvalue (Variables|/Script/Starbreeze.PD3HeistDataAsset|GetHeistDisplayName (.HeistData (Utilities|Struct|BreakSBZHeistDataLevelPair _array_element))))
    ;[0 0 0] Possibly add best time here
    (Default|SetTextDescription _returnvalue)
    (if (Utilities|IsValidSoftObjectReference (Variables|/Script/Starbreeze.PD3HeistDataAsset|GetHeistBannerImage (.HeistData (Utilities|Struct|BreakSBZHeistDataLevelPair _array_element))))
      (bind _returnvalue_2 (Utilities|LoadAssetBlocking (Variables|/Script/Starbreeze.PD3HeistDataAsset|GetHeistBannerImage (.HeistData (Utilities|Struct|BreakSBZHeistDataLevelPair _array_element)))))
      (bind _aspaper_sprite (Utilities|Casting|CastToPaperSprite _returnvalue_2))
      (Variables|/Game/UI/Widgets/Menus/Buttons/WBP_UI_CrimeNet_TextButton.WBP_UI_CrimeNet_TextButton_C|SetPaperSprite_Image_Buttons _returnvalue _aspaper_sprite)
      (else
        (Variables|/Game/UI/Widgets/Menus/Buttons/WBP_UI_CrimeNet_TextButton.WBP_UI_CrimeNet_TextButton_C|SetPaperSprite_Image_Buttons _returnvalue "/Game/Mods/_NadzMods/ModdedHeistSelectionMenu/UI/Textures/SS_UI_Placeholder_Banner_Sprite.SS_UI_Placeholder_Banner_Sprite")))
    (Layout|BorderSlot|SetPadding _returnvalue (Utilities|Struct|MakeMargin 0.0 0.0 0.0 5.0) :!class /Script/UMG.UserWidget)
    (EventDispatchers|BindEventtoOnButtonSelected _returnvalue (EventDispatchers|CreateEvent :!event Custom|OnHeistButtonSelected))
    (EventDispatchers|BindEventtoOnButtonFocusedChanged _returnvalue (EventDispatchers|CreateEvent :!event Custom|OnButtonHover))
    (Utilities|Map|Add (Variables|Default|GetHeistDataButtonsMap) _returnvalue _array_element)))

(fn SetSelectedHeistInfo
  (params (SelectedButton :type WBP%20UI%20Crime%20Net%20Text%20Button%20Object%20Reference))
  (bind _heistdatabuttonsmap (Variables|Default|GetHeistDataButtonsMap))
  (bind _value (Utilities|Map|Find _heistdatabuttonsmap SelectedButton))
  (bind (_heistdata _levelpath) (Utilities|Struct|BreakSBZHeistDataLevelPair _value))
  (|SetStealthTimeTextToArray)
  (|SetLoudTimeTextToArray)
  (Utilities|Array|Clear (Variables|Default|GetStealthTimes))
  (Utilities|Array|Clear (Variables|Default|GetLoudTimes))
  (Rendering|Components|TextRender|SetText (Variables|Default|GetText_Desc_LevelDescription) (Variables|/Script/Starbreeze.PD3HeistDataAsset|GetHeistDescription _heistdata))
  (for _array_element (Class|SBZPlayerStatisticsManager|GetHeistBestTimes (Class|SBZPlayerStatisticsManager|GetPlayerStatisticsManager) _levelpath)
    (Utilities|Array|Add (Variables|Default|GetStealthTimes) (Utilities|String|ToString(Float) (.StealthTime (Utilities|Struct|BreakSBZLevelTimesStruct _array_element))))
    (Utilities|Array|Add (Variables|Default|GetLoudTimes) (Utilities|String|ToString(Float) (.LoudTime (Utilities|Struct|BreakSBZLevelTimesStruct _array_element))))
    (for (_array_element_2 _array_index) (LocalVariables|GetStealthTimeText)
      (if (== (Math|Conversions|ToFloat(Integer) (Utilities|Array|Get(acopy) (Variables|Default|GetStealthTimes) _array_index)) -1.0)
        (Rendering|Components|TextRender|SetText _array_element_2 "N/A")
        (else
          (bind _returnvalue (Class|SBZUIStatics|FormatInttoTimerText (Math|Float|Truncate (Math|Conversions|ToFloat(Integer) (Utilities|Array|Get(acopy) (Variables|Default|GetStealthTimes) _array_index))) false))
          (Rendering|Components|TextRender|SetText _array_element_2 _returnvalue)))
      (for (_array_element_3 _array_index_2) (LocalVariables|GetLoudTimeText)
        (if (== (Math|Conversions|ToFloat(Integer) (Utilities|Array|Get(acopy) (Variables|Default|GetLoudTimes) _array_index_2)) -1.0)
          (Rendering|Components|TextRender|SetText _array_element_3 "N/A")
          (else
            (bind _returnvalue_2 (Class|SBZUIStatics|FormatInttoTimerText (Math|Float|Truncate (Math|Conversions|ToFloat(Integer) (Utilities|Array|Get(acopy) (Variables|Default|GetLoudTimes) _array_index_2))) false))
            (Rendering|Components|TextRender|SetText _array_element_3 _returnvalue_2)))))))

(fn GetMainMenuCrimenet)