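; Blueprint function library for the PD3 mod loader's Settings Manager, handling per-mod settings, mod metadata lookup and widget re-parenting.
; Settings live in one save slot per mod name, and LoadSettings creates a missing save and re-saves on every load.
; Typed getters reload the save on each call, logging and returning a fallback for missing keys.
; Reconstruct helpers re-add widgets to overlay or canvas panels, reapplying captured slot layout.
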(fn ReconstructOverlayWidget
  (params (Overlay :type Overlay%20Object%20Reference) (Widget :type Widget%20Object%20Reference) (__WorldContext :type Object%20Object%20Reference))
  (bind _returnvalue (Class|WidgetLayoutLibrary|SlotasOverlaySlot Overlay))
  (Utilities|FlowControl|Sequence
    (:then_0
      (LocalVariables|SetHAlignment (Variables|/Script/UMG.OverlaySlot|GetHorizontalAlignment _returnvalue))
      (LocalVariables|SetPadding (Variables|/Script/UMG.OverlaySlot|GetPadding _returnvalue))
      (LocalVariables|SetVAlignment (Variables|/Script/UMG.OverlaySlot|GetVerticalAlignment _returnvalue)))
    (:then_1
      (Widget|RemovefromParent Widget)
      (bind _returnvalue_2 (Class|Overlay|AddChildtoOverlay Overlay Widget))
      (Layout|GridSlot|SetHorizontalAlignment _returnvalue_2 (LocalVariables|GetHAlignment))
      (Layout|GridSlot|SetVerticalAlignment _returnvalue_2 (LocalVariables|GetVAlignment))
      (Layout|BorderSlot|SetPadding _returnvalue_2 (LocalVariables|GetPadding) :!class /Script/UMG.OverlaySlot))))

(fn ReconstructCanvasWidget
  (params (CanvasPanel :type Canvas%20Panel%20Object%20Reference) (Widget :type Widget%20Object%20Reference))
  (bind _returnvalue (Class|WidgetLayoutLibrary|SlotasCanvasSlot Widget))
  (Utilities|FlowControl|Sequence
    (:then_0
      (LocalVariables|SetAutoSize (Class|CanvasPanelSlot|GetAutoSize _returnvalue))
      (LocalVariables|SetLayout (Class|CanvasPanelSlot|GetLayout _returnvalue))
      (LocalVariables|SetSize (Class|CanvasPanelSlot|GetSize _returnvalue))
      (LocalVariables|SetPosition (Class|CanvasPanelSlot|GetPosition _returnvalue)))
    (:then_1
      (Widget|RemovefromParent Widget)
      (bind _returnvalue_2 (Class|CanvasPanel|AddChildtoCanvas CanvasPanel Widget))
      (Class|CanvasPanelSlot|SetAutoSize _returnvalue_2 (LocalVariables|GetAutoSize))
      (Class|CanvasPanelSlot|SetLayout _returnvalue_2 (LocalVariables|GetLayout))
      (Class|CanvasPanelSlot|SetSize _returnvalue_2 (LocalVariables|GetSize))
      (Class|CanvasPanelSlot|SetPosition _returnvalue_2 (LocalVariables|GetPosition)))))

(fn SaveSettings
  (params (ModName :type String) (SaveGameObject :type Save%20Game%20Object%20Reference))
  (SaveGame|SaveGametoSlot SaveGameObject (CallFunction|MakeSlotNamefromModName ModName)))

(fn LoadSettings
  (params (ModName :type String))
  (bind _slotname (CallFunction|MakeSlotNamefromModName ModName))
  (bind _returnvalue (SaveGame|DoesSaveGameExist _slotname))
  (if _returnvalue
    (bind _returnvalue_2 (SaveGame|LoadGamefromSlot _slotname))
    (bind _asbp_settings_manger_save_game (Utilities|Casting|CastToBP_SettingsManger_SaveGame _returnvalue_2))
    (Save|SaveSettings ModName _asbp_settings_manger_save_game)
    (return _asbp_settings_manger_save_game)
    (else
      (bind _returnvalue_3 (SaveGame|CreateSaveGameObject "/Game/Mods/ModLoader/Extensions/Blueprints/SettingsManager/BP_SettingsManger_SaveGame.BP_SettingsManger_SaveGame_C"))
      (Save|SaveSettings ModName _returnvalue_3)
      (return _returnvalue_3))))

(fn GetModMeta
  (params (ModID :type Name))
  (bind _parsedmoddata (ModData|GetAllModMetas))
  (for _array_element _parsedmoddata
    (if (Utilities|Name|Equal(Name) (Variables|/Game/Mods/ModLoader/Blueprints/PDA_ModMeta.PDA_ModMeta_C|GetModID _array_element) ModID)
      (return _array_element))))

(fn MakeSlotNamefromModName
  (params (ModName :type String))
  (return (Utilities|String|Append "Mod_Setting_" ModName)))

(fn GetAllModMetas
  (bind _aspd3_game_instance (Utilities|Casting|CastToPD3_GameInstance (Game|GetGameInstance)))
  (bind _modloadermanagerinstance (CallFunction|GetModLoaderManager _aspd3_game_instance))
  (return (Variables|/Game/Mods/ModLoader/Blueprints/ModLoaderManager.ModLoaderManager_C|GetParsedModData _modloadermanagerinstance)))

(fn GetSettingsFloat
  (params (ModName :type String) (SettingsName :type String))
  (bind _returnvalue (Save|LoadSettings ModName))
  (if (.ReturnValue (Utilities|Map|Find (.floatsettings (Variables|/Game/Mods/ModLoader/Extensions/Blueprints/SettingsManager/BP_SettingsManger_SaveGame.BP_SettingsManger_SaveGame_C|GetSettings _returnvalue)) SettingsName))
    (return (.Value (Utilities|Map|Find (.floatsettings (Variables|/Game/Mods/ModLoader/Extensions/Blueprints/SettingsManager/BP_SettingsManger_SaveGame.BP_SettingsManger_SaveGame_C|GetSettings _returnvalue)) SettingsName)))
    (else
      (CallFunction|PrinttoModLoader (Utilities|String|Append SettingsName " value not found"))
      (return -1.0))))

(fn GetSettingsBool
  (params (ModName :type String) (SettingsName :type String) (__WorldContext :type Object%20Object%20Reference))
  (bind _returnvalue (Save|LoadSettings ModName))
  (if (.ReturnValue (Utilities|Map|Find (.boolsettings (Variables|/Game/Mods/ModLoader/Extensions/Blueprints/SettingsManager/BP_SettingsManger_SaveGame.BP_SettingsManger_SaveGame_C|GetSettings _returnvalue)) SettingsName))
    (return (.Value (Utilities|Map|Find (.boolsettings (Variables|/Game/Mods/ModLoader/Extensions/Blueprints/SettingsManager/BP_SettingsManger_SaveGame.BP_SettingsManger_SaveGame_C|GetSettings _returnvalue)) SettingsName)))
    (else
      (CallFunction|PrinttoModLoader (Utilities|String|Append SettingsName " value not found"))
      (return false))))

(fn GetSettingsVector2D
  (params (ModName :type String) (SettingsName :type String) (__WorldContext :type Object%20Object%20Reference))
  (bind _returnvalue (Save|LoadSettings ModName))
  (if (.ReturnValue (Utilities|Map|Find (.vector2dsettings (Variables|/Game/Mods/ModLoader/Extensions/Blueprints/SettingsManager/BP_SettingsManger_SaveGame.BP_SettingsManger_SaveGame_C|GetSettings _returnvalue)) SettingsName))
    (return (.Value (Utilities|Map|Find (.vector2dsettings (Variables|/Game/Mods/ModLoader/Extensions/Blueprints/SettingsManager/BP_SettingsManger_SaveGame.BP_SettingsManger_SaveGame_C|GetSettings _returnvalue)) SettingsName)))
    (else
      (CallFunction|PrinttoModLoader (Utilities|String|Append SettingsName " value not found"))
      (return "(X=-1.000000,Y=-1.000000)"))))

(fn GetSettingsVector3D
  (params (ModName :type String) (SettingsName :type String) (__WorldContext :type Object%20Object%20Reference))
  (bind _returnvalue (Save|LoadSettings ModName))
  (if (.ReturnValue (Utilities|Map|Find (.vector3dsettings (Variables|/Game/Mods/ModLoader/Extensions/Blueprints/SettingsManager/BP_SettingsManger_SaveGame.BP_SettingsManger_SaveGame_C|GetSettings _returnvalue)) SettingsName))
    (return (.Value (Utilities|Map|Find (.vector3dsettings (Variables|/Game/Mods/ModLoader/Extensions/Blueprints/SettingsManager/BP_SettingsManger_SaveGame.BP_SettingsManger_SaveGame_C|GetSettings _returnvalue)) SettingsName)))
    (else
      (CallFunction|PrinttoModLoader (Utilities|String|Append SettingsName " value not found"))
      (return "-1.000000,-1.000000,-1.000000"))))

(fn GetSettingsColor
  (params (ModName :type String) (SettingsName :type String) (__WorldContext :type Object%20Object%20Reference))
  (bind _returnvalue (Save|LoadSettings ModName))
  (if (.ReturnValue (Utilities|Map|Find (.colorsettings (Variables|/Game/Mods/ModLoader/Extensions/Blueprints/SettingsManager/BP_SettingsManger_SaveGame.BP_SettingsManger_SaveGame_C|GetSettings _returnvalue)) SettingsName))
    (return (.Value (Utilities|Map|Find (.colorsettings (Variables|/Game/Mods/ModLoader/Extensions/Blueprints/SettingsManager/BP_SettingsManger_SaveGame.BP_SettingsManger_SaveGame_C|GetSettings _returnvalue)) SettingsName)))
    (else
      (CallFunction|PrinttoModLoader (Utilities|String|Append SettingsName " value not found"))
      (return ""))))

(fn GetSettingsInput
  (params (ModName :type String) (SettingsName :type String) (__WorldContext :type Object%20Object%20Reference))
  (bind _returnvalue (Save|LoadSettings ModName))
  (if (.ReturnValue (Utilities|Map|Find (.inputsettings (Variables|/Game/Mods/ModLoader/Extensions/Blueprints/SettingsManager/BP_SettingsManger_SaveGame.BP_SettingsManger_SaveGame_C|GetSettings _returnvalue)) SettingsName))
    (return (.Value (Utilities|Map|Find (.inputsettings (Variables|/Game/Mods/ModLoader/Extensions/Blueprints/SettingsManager/BP_SettingsManger_SaveGame.BP_SettingsManger_SaveGame_C|GetSettings _returnvalue)) SettingsName)))
    (else
      (CallFunction|PrinttoModLoader (Utilities|String|Append SettingsName " value not found"))
      (return ""))))