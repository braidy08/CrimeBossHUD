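; BP_SettingsManager is a mod loader extension actor that injects mod settings categories into the in-game action phase menu.
; On BeginPlay it finds the settings manager widget among the mod loader's extensions, then collapses and initializes each category widget.
; Each category is added as a nav button to every action phase menu widget found.
; Its name and "Settings_"-prefixed stack key come from the manager's category map.
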(event EventBeginPlay
  (bind _modloadermanagerinstance (CallFunction|GetModLoaderManager))
  (for _array_element (Variables|/Game/Mods/ModLoader/Blueprints/ModLoaderManager.ModLoaderManager_C|GetMLExtensions _modloadermanagerinstance)
    (bind _aswbp_mlextension_widget_settings_manager (Utilities|Casting|CastToWBP_MLExtensionWidget_SettingsManager _array_element))
    (bind _output_get (Variables|Default|SetSettingsManager _aswbp_mlextension_widget_settings_manager))
    (for _array_element_2 (Variables|/Game/Mods/ModLoader/Extensions/Blueprints/SettingsManager/WBP_MLExtensionWidget_SettingsManager.WBP_MLExtensionWidget_SettingsManager_C|GetSettingsCategoryWidgets _output_get)
      (Widget|SetVisibility _array_element_2 "Collapsed")
      (Class|SBZSettingsCategoryScreen|SettingsCategoryInitialized _array_element_2)
      ;[0.02604 0.02604 0.02604] Add Button to Menu
      (bind _foundwidgets (Widget|GetAllWidgetsOfClass "/Game/UI/Widgets/StateMachine/ActionPhase/WBP_UI_SM_ActionPhaseMenu.WBP_UI_SM_ActionPhaseMenu_C" false))
      (for _array_element_3 _foundwidgets
        (Default|AddSettingtoMenu (Variables|Default|GetSettingsManager) _array_element_3 _array_element_2 (Utilities|Struct|MakeSBZNavButtonParameters (Utilities|String|StringToName (Utilities|String|Append "Settings_" (Utilities|String|ToString(Name) (.CategoryName (Utilities|Struct|BreakSBZSettingsMenuCategoryInfo (.Value (Utilities|Map|Find (Variables|/Game/Mods/ModLoader/Extensions/Blueprints/SettingsManager/WBP_MLExtensionWidget_SettingsManager.WBP_MLExtensionWidget_SettingsManager_C|GetModSettingsCategories _output_get) (Utilities|String|ToString(Name) (Variables|/Game/UI/Widgets/Menus/Settings/WBP_Settings_Screen_Category.WBP_Settings_Screen_Category_C|GetSettingsCategoryName _array_element_2))))))))) (Utilities|Text|ToText(String) (Utilities|String|ToString(Name) (.CategoryName (Utilities|Struct|BreakSBZSettingsMenuCategoryInfo (.Value (Utilities|Map|Find (Variables|/Game/Mods/ModLoader/Extensions/Blueprints/SettingsManager/WBP_MLExtensionWidget_SettingsManager.WBP_MLExtensionWidget_SettingsManager_C|GetModSettingsCategories _output_get) (Utilities|String|ToString(Name) (Variables|/Game/UI/Widgets/Menus/Settings/WBP_Settings_Screen_Category.WBP_Settings_Screen_Category_C|GetSettingsCategoryName _array_element_2))))))))))
        (Variables|/Game/UI/Widgets/Menus/Settings/WBP_Settings_Screen_Category.WBP_Settings_Screen_Category_C|SetSettingsCategoryName _array_element_2 (.CategoryName (Utilities|Struct|BreakSBZSettingsMenuCategoryInfo (.Value (Utilities|Map|Find (Variables|/Game/Mods/ModLoader/Extensions/Blueprints/SettingsManager/WBP_MLExtensionWidget_SettingsManager.WBP_MLExtensionWidget_SettingsManager_C|GetModSettingsCategories _output_get) (Utilities|String|ToString(Name) (Variables|/Game/UI/Widgets/Menus/Settings/WBP_Settings_Screen_Category.WBP_Settings_Screen_Category_C|GetSettingsCategoryName _array_element_2)))))))
        (Variables|/Script/Starbreeze.SBZMenuStackWidget|SetStackValue _array_element_2 (Utilities|String|StringToName (Utilities|String|Append "Settings_" (Utilities|String|ToString(Name) (.CategoryName (Utilities|Struct|BreakSBZSettingsMenuCategoryInfo (.Value (Utilities|Map|Find (Variables|/Game/Mods/ModLoader/Extensions/Blueprints/SettingsManager/WBP_MLExtensionWidget_SettingsManager.WBP_MLExtensionWidget_SettingsManager_C|GetModSettingsCategories _output_get) (Utilities|String|ToString(Name) (Variables|/Game/UI/Widgets/Menus/Settings/WBP_Settings_Screen_Category.WBP_Settings_Screen_Category_C|GetSettingsCategoryName _array_element_2))))))))))))))

(fn ConstructionScript
  (|CallParentFunction))